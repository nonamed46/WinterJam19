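; Destructible box that drifts in the moving world around the ship, awarding the player score when a Ship_BP overlaps it.
; The construction script randomizes its initial drift, height, rotation and scale.
; Through MovingWorld_BPI it receives the player direction, and a looping timer offsets the box by that plus its drift.
; Ship overlap removes the Box component, and either overlap or fracture sets a delayed self-destruct.
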(event OnComponentBeginOverlap(Box)
  (params (OverlappedComponent :type Primitive%20Component%20Object%20Reference) (OtherActor :type Actor%20Object%20Reference) (OtherComp :type Primitive%20Component%20Object%20Reference) (OtherBodyIndex :type Integer) (bFromSweep :type Boolean) (SweepResult :type Hit%20Result%20Structure%20%28by%20ref%29))
  ;[1 1 1] When Character Overlaps: Increase Score and SelfDestruct after x seconds.
  (Utilities|Casting|CastToShip_BP OtherActor)
  (bind _astop_down_character (Utilities|Casting|CastToTopDownCharacter (Game|GetPlayerCharacter 0)))
  (Default|IncreaseScore _astop_down_character 10)
  (Components|DestroyComponent (Variables|Default|GetBox))
  (Actor|SetLifeSpan 2e+01))

(event OnComponentFracture(Destructible)
  (params (HitPoint :type Vector%20%28by%20ref%29 :default "0, 0, 0") (HitDirection :type Vector%20%28by%20ref%29 :default "0, 0, 0"))
  ;[1 1 1] When Character Overlaps: Increase Score and SelfDestruct after x seconds.
  (Actor|SetLifeSpan 2e+01))

(event Custom|Move
  (bind _initialdirection (Variables|Default|GetInitialDirection))
  (bind _playerdirection (Variables|Default|GetPlayerDirection))
  (bind _returnvalue (+ _playerdirection _initialdirection))
  ;[1 1 1] Called by StartMoving
  (Transformation|AddActorLocalOffset (Math|Vector|MakeVector (.x _returnvalue) (.y _returnvalue) 0.0) false false))

(event EventStartMoving
  ;[1 1 1] Called via MovingWorld_BPI from the ShipBP.
  ;;[1 1 1] Starts/StopsMoving
  (Utilities|FlowControl|DoOnce false
    (:Completed
      (Utilities|Time|SetTimerbyEvent (delegate Custom|Move) 0.05 true))))

(event EventStopMoving
  ;[1 1 1] Called via MovingWorld_BPI from the ShipBP.
  ;;[1 1 1] Starts/StopsMoving
  (Utilities|Time|SetTimerbyEvent (delegate Custom|Move) 0.0)
  (Utilities|FlowControl|DoOnce false) ; enters at Reset
)

(event EventSetPlayerDirection
  (params (PlayerDirection :type Vector :default "0, 0, 0"))
  ;[1 1 1] Called via MovingWorld_BPI from the ShipBP.
  ;;[1 1 1] Get the PlayerDirection from the Interface and Save it as Var
  (Variables|Default|SetPlayerDirection PlayerDirection))

(fn ConstructionScript
  (bind _maxinitialspeed (Variables|Default|GetMaxInitialSpeed))
  (bind _destructible (Variables|Default|GetDestructible))
  (bind _returnvalue (Transformation|GetWorldLocation _destructible))
  (bind _returnvalue_2 (* _maxinitialspeed -1.0))
  (Variables|Default|SetInitialDirection (Math|Vector|MakeVector (Math|Random|RandomFloatinRange _returnvalue_2 _maxinitialspeed) (Math|Random|RandomFloatinRange _returnvalue_2 _maxinitialspeed) 0.0))
  (Transformation|SetWorldTransform _destructible (Math|Transform|MakeTransform (Math|Vector|MakeVector (.x _returnvalue) (.y _returnvalue) (+ (.z _returnvalue) (Math|Random|RandomFloatinRange -2e+01 -5.0))) (Math|Rotator|MakeRotator (Math|Random|RandomFloatinRange -2e+01 2e+01) (Math|Random|RandomFloatinRange -2e+01 2e+01) (Math|Random|RandomFloatinRange -2e+01 2e+01)) (* (Math|Vector|MakeVector (Math|Random|RandomFloatinRange 0.85 1.1) (Math|Random|RandomFloatinRange 0.85 1.1) (Math|Random|RandomFloatinRange 0.85 1.1)) (Math|Random|RandomFloatinRange 0.85 1.1))) false false))