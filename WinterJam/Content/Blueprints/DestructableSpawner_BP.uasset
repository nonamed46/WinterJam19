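; Spawner actor that scatters destructible boxes, barrels and boats around itself at BeginPlay.
; SpawnDestructibles loops a set count, taking a weighted random class that favors boxes and barrels, plus a location from FreeSpawnLocation.
; That function recursively retries random offsets, testing minimum spacing against CurrentSpawnLocations up to a depth limit.
; The random offset is re-rolled between check, store and return, so spacing is not guaranteed.
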(event Custom|SpawnDestructibles
  (params (Amount :type Integer))
  ;[1 1 1] Reset Array then Loop x Times. Each loop get a random Class and Location and check if you can spawn. If so then Spawn that actor with the calculated values.
  (Variables|Default|SetCurrentSpawnLocations (Utilities|Array|MakeArray))
  (for _index (range 1 Amount)
    (bind (_destructibleclass _spawnlocation _canspawn_) (CallFunction|RandomClassandLocation))
    (if _canspawn_
      (Game|SpawnActorfromClass _destructibleclass (Math|Transform|MakeTransform _spawnlocation (Transformation|GetWorldRotation (Variables|Default|GetDefaultSceneRoot)) "1,1,1") "AdjustIfPossibleButDontSpawnIfColliding" 0 0)
      (Development|PrintString "a new swanky actor has been spawned")
      (else
        (Development|PrintString "Unable to spawn :( not enough space!"))))
  (bind _outactors (Actor|GetAllActorsOfClass "/Game/Blueprints/DestBox_p_BP.DestBox_p_BP_C"))
  (Development|PrintString (Utilities|String|Append "Done Spawning: " (Utilities|String|ToString(Integer) (Utilities|Array|Length _outactors)) " Actors spawned Correctly")))

(event EventBeginPlay
  (CallFunction|SpawnDestructibles 20))

(fn ConstructionScript)

(fn RandomClassandLocation
  ;[1 1 1] Gets an empty location to spawn and calculates based on weighted bools which Destructibles to spawn. Returns Class Location and validity of the action
  (bind (_location _foundlocation_) (CallFunction|FreeSpawnLocation 0.0))
  (if (Math|Random|RandomBoolwithWeight 0.8)
    (if (Math|Random|RandomBool)
      (return "/Game/Blueprints/DestBox_p_BP.DestBox_p_BP_C" _location _foundlocation_)
      (else
        (return "/Game/Blueprints/DestBarrel_c_BP.DestBarrel_c_BP_C" _location _foundlocation_)))
    (else
      (return "/Game/Blueprints/DestBoat_c_BP.DestBoat_c_BP_C" _location _foundlocation_))))

(fn FreeSpawnLocation
  (params (recDepth :type Float%20%28single-precision%29))
  (bind _returnvalue (Transformation|GetActorLocation))
  (bind _returnvalue_2 (Math|Random|RandomUnitVector))
  (bind _returnvalue_3 (* _returnvalue_2 "1000.000000,1000.000000,1.000000"))
  (bind _returnvalue_4 (+ _returnvalue_3 _returnvalue))
  ;[1 1 1] If the random location is in empty space add it to the Spawn Locations array and return Location. Else try again until it failed 15 times
  (if (< recDepth 15.0)
    (bind _emptyspace (CallFunction|IsSpaceEmpty? _returnvalue_4))
    (if _emptyspace
      (Utilities|Array|Add (Variables|Default|GetCurrentSpawnLocations) _returnvalue_4)
      (return _returnvalue_4 true)
      (else
        (bind (_location _foundlocation_) (CallFunction|FreeSpawnLocation (+ recDepth 1.0)))
        (return _location _foundlocation_)))
    (else
      (return "0, 0, 0" false))))

(fn IsSpaceEmpty?
  (params (Space :type Vector))
  ;[1 1 1] Checks if the Location is further away than MinSpawnDistance
  (for _array_element (Variables|Default|GetCurrentSpawnLocations)
    (if (< (Math|Vector|VectorLength (- _array_element Space)) (Variables|Default|GetMinSpawnDistance))
      (return false)))
  (return true))