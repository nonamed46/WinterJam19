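; Destructible world object that drifts and awards score to the TopDownCharacter when the ship overlaps it.
; The ship passes its direction through MovingWorld_BPI, and a looping timer offsets the actor by that plus a random drift set in the Construction Script.
; StartMoving and StopMoving toggle the timer through a resettable DoOnce.
; Overlap with Ship_BP removes the collision box and schedules delayed self-destruction.
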(event OnComponentBeginOverlap(Box)
  (params (OverlappedComponent :type Primitive%20Component%20Object%20Reference) (OtherActor :type Actor%20Object%20Reference) (OtherComp :type Primitive%20Component%20Object%20Reference) (OtherBodyIndex :type Integer) (bFromSweep :type Boolean) (SweepResult :type Hit%20Result%20Structure%20%28by%20ref%29))
  ;[1 1 1] When Character Overlaps: Increase Score and SelfDestruct after x seconds.
  (Utilities|Casting|CastToShip_BP OtherActor)
  (bind _astop_down_character (Utilities|Casting|CastToTopDownCharacter (Game|GetPlayerCharacter 0)))
  (Default|IncreaseScore _astop_down_character 10)
  (Components|DestroyComponent (Variables|Default|GetBox))
  (Utilities|Time|SetTimerbyEvent (delegate Custom|SelfDestruct) 2e+01))

(event Custom|SelfDestruct
  ;[1 1 1] When Character Overlaps: Increase Score and SelfDestruct after x seconds.
  (Development|PrintString "Me is ded")
  (Actor|DestroyActor))

(event Custom|Move
  (bind _initialdirection (Variables|Default|GetInitialDirection))
  (bind _playerdirection (Variables|Default|GetPlayerDirection))
  (bind _returnvalue (+ _playerdirection _initialdirection))
  ;[1 1 1] Called by StartMoving
  (Transformation|AddActorLocalOffset (Math|Vector|MakeVector (.x _returnvalue) (.y _returnvalue) 0.0) false false))

(event EventStartMoving
  ;[1 1 1] Called via MovingWorld_BPI from the ShipBP.
  ;;[1 1 1] Starts/StopsMoving
  (Utilities|FlowControl|DoOnce false
    (:Completed
      (Utilities|Time|SetTimerbyEvent (delegate Custom|Move) 0.05 true))))

(event EventStopMoving
  ;[1 1 1] Called via MovingWorld_BPI from the ShipBP.
  ;;[1 1 1] Starts/StopsMoving
  (Utilities|Time|SetTimerbyEvent (delegate Custom|Move) 0.0)
  (Utilities|FlowControl|DoOnce false) ; enters at Reset
)

(event EventSetPlayerDirection
  (params (PlayerDirection :type Vector :default "0, 0, 0"))
  ;[1 1 1] Called via MovingWorld_BPI from the ShipBP.
  ;;[1 1 1] Get the PlayerDirection from the Interface and Save it as Var
  (Variables|Default|SetPlayerDirection PlayerDirection))

(fn ConstructionScript
  (bind _maxinitialspeed (Variables|Default|GetMaxInitialSpeed))
  (bind _returnvalue (* _maxinitialspeed -1.0))
  (Variables|Default|SetInitialDirection (Math|Vector|MakeVector (Math|Random|RandomFloatinRange _returnvalue _maxinitialspeed) (Math|Random|RandomFloatinRange _returnvalue _maxinitialspeed) 0.0)))