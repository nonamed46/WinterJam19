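; Enemy spawner actor that periodically creates EnemyCharacter AI at its own location and sends each toward the player.
; BeginPlay starts a looping five-second timer only if the level holds no more than 20 enemies; the count is never rechecked afterward.
; Each timer tick spawns an enemy and, if valid, issues a Simple Move To Actor targeting the first player character.
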(event Custom|SpawnAI
  (bind _returnvalue (AI|SpawnAIFromClass "/Game/TopDownBP/Blueprints/EnemyCharacter.EnemyCharacter_C" 0 (Transformation|GetActorLocation self) "0, 0, 0" false))
  (Utilities|IsValid _returnvalue
    (:Is%20Valid
      (AI|Navigation|SimpleMovetoActor (Pawn|GetController _returnvalue) (Game|GetPlayerCharacter 0)))))

(event EventBeginPlay
  (bind _outactors (Actor|GetAllActorsOfClass "/Game/TopDownBP/Blueprints/EnemyCharacter.EnemyCharacter_C"))
  (if (<= (Utilities|Array|Length _outactors) 20)
    (Utilities|Time|SetTimerbyEvent (delegate Custom|SpawnAI) 5.0 true)))

(fn ConstructionScript)