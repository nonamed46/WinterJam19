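; Island spawner actor that places randomly chosen island actors at its location with a random horizontal offset.
; It spawns one of eight island classes on BeginPlay and remembers it as LastSpawnedIsland.
; A timer, looping only when ShouldRespawn is set, spawns another once the last island is destroyed or has moved beyond a set distance from the spawner.
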(event Custom|SpawnRandomIsland
  (bind _returnvalue (Math|Random|RandomFloatinRange -4e+02 4e+02))
  (bind _returnvalue_2 (Math|Random|RandomFloatinRange -4e+02 4e+02))
  (bind _defaultsceneroot (Variables|Default|GetDefaultSceneRoot))
  (bind _returnvalue_3 (Transformation|GetWorldLocation _defaultsceneroot))
  (bind _returnvalue_4 (+ (.y _returnvalue_3) _returnvalue))
  (bind _returnvalue_5 (+ (.x _returnvalue_3) _returnvalue_2))
  (bind _returnvalue_6 (Math|Transform|MakeTransform (Math|Vector|MakeVector _returnvalue_5 _returnvalue_4 (.z _returnvalue_3))))
  (switch int (Math|Random|RandomInteger 8)
    (:Default
      (bind _returnvalue_7 (Game|SpawnActorfromClass "/Game/Blueprints/Islands/Island01_cBP.Island01_cBP_C" _returnvalue_6 "AlwaysSpawn" 0 0 :!label _label))
      (Variables|Default|SetLastSpawnedIsland _returnvalue_7))
    (:0
      (goto _label))
    (:1
      (bind _returnvalue_8 (Game|SpawnActorfromClass "/Game/Blueprints/Islands/Island02_cBP.Island02_cBP_C" _returnvalue_6 "AlwaysSpawn" 0 0))
      (Variables|Default|SetLastSpawnedIsland _returnvalue_8))
    (:2
      (bind _returnvalue_9 (Game|SpawnActorfromClass "/Game/Blueprints/Islands/Island03_cBP.Island03_cBP_C" _returnvalue_6 "AlwaysSpawn" 0 0))
      (Variables|Default|SetLastSpawnedIsland _returnvalue_9))
    (:3
      (bind _returnvalue_10 (Game|SpawnActorfromClass "/Game/Blueprints/Islands/Island04_cBP.Island04_cBP_C" _returnvalue_6 "AlwaysSpawn" 0 0))
      (Variables|Default|SetLastSpawnedIsland _returnvalue_10))
    (:4
      (bind _returnvalue_11 (Game|SpawnActorfromClass "/Game/Blueprints/Islands/Island05_cBP.Island05_cBP_C" _returnvalue_6 "AlwaysSpawn" 0 0))
      (Variables|Default|SetLastSpawnedIsland _returnvalue_11))
    (:5
      (bind _returnvalue_12 (Game|SpawnActorfromClass "/Game/Blueprints/Islands/Island06_cBP.Island06_cBP_C" _returnvalue_6 "AlwaysSpawn" 0 0))
      (Variables|Default|SetLastSpawnedIsland _returnvalue_12))
    (:6
      (bind _returnvalue_13 (Game|SpawnActorfromClass "/Game/Blueprints/Islands/Island07_cBP.Island07_cBP_C" _returnvalue_6 "AlwaysSpawn" 0 0))
      (Variables|Default|SetLastSpawnedIsland _returnvalue_13))
    (:7
      (bind _returnvalue_14 (Game|SpawnActorfromClass "/Game/Blueprints/Islands/Island08_cBP.Island08_cBP_C" _returnvalue_6 "AlwaysSpawn" 0 0))
      (Variables|Default|SetLastSpawnedIsland _returnvalue_14))))

(event Custom|RespawnTimer
  (bind _lastspawnedisland (Variables|Default|GetLastSpawnedIsland))
  (Utilities|IsValid _lastspawnedisland
    (:Is%20Valid
      (if (> (Transformation|GetDistanceTo _lastspawnedisland self) 4e+03)
        (CallFunction|SpawnRandomIsland :!label _label)))
    (:Is%20Not%20Valid
      (goto _label))))

(event EventBeginPlay
  (CallFunction|SpawnRandomIsland)
  (Utilities|Time|SetTimerbyEvent (delegate Custom|RespawnTimer) 2.0 (Variables|Default|GetShouldRespawn)))

(fn ConstructionScript)