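; Island actor for a moving-world setup, shifting itself by a player direction supplied from the ShipBP through MovingWorld_BPI.
; The Construction Script picks one of three island meshes and randomizes its yaw and non-uniform scale for variety.
; StartMoving uses a DoOnce to start a looping timer that offsets the actor along the stored direction's X and Y; StopMoving clears the timer and resets the gate.
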(event Custom|Move
  (bind _playerdirection (Variables|Default|GetPlayerDirection))
  ;[1 1 1] Called by StartMoving
  (Transformation|AddActorLocalOffset (Math|Vector|MakeVector (.x _playerdirection) (.y _playerdirection) 0.0) false false))

(event EventStartMoving
  ;[1 1 1] Called via MovingWorld_BPI from the ShipBP.
  ;;[1 1 1] Starts/StopsMoving
  (Utilities|FlowControl|DoOnce false
    (:Completed
      (Utilities|Time|SetTimerbyEvent (delegate Custom|Move) 0.05 true))))

(event EventStopMoving
  ;[1 1 1] Called via MovingWorld_BPI from the ShipBP.
  ;;[1 1 1] Starts/StopsMoving
  (Utilities|Time|SetTimerbyEvent (delegate Custom|Move) 0.0)
  (Utilities|FlowControl|DoOnce false) ; enters at Reset
)

(event EventSetPlayerDirection
  (params (PlayerDirection :type Vector :default "0, 0, 0"))
  ;[1 1 1] Called via MovingWorld_BPI from the ShipBP.
  ;;[1 1 1] Get the PlayerDirection from the Interface and Save it as Var
  (Variables|Default|SetPlayerDirection PlayerDirection))

(fn ConstructionScript
  (bind _staticmesh (Variables|Default|GetStaticMesh))
  (switch int (Math|Random|RandomIntegerinRange 0 2)
    (:Default
      (Components|StaticMesh|SetStaticMesh _staticmesh "/Game/Assets/island01.island01" :!label _label))
    (:0
      (goto _label))
    (:1
      (Components|StaticMesh|SetStaticMesh _staticmesh "/Game/Assets/island02.island02"))
    (:2
      (Components|StaticMesh|SetStaticMesh _staticmesh "/Game/Assets/island03.island03")))
  (Transformation|AddLocalRotation _staticmesh (Math|Rotator|MakeRotator 0.0 0.0 (Math|Random|RandomFloatinRange 0.0 359.899994)) false false)
  (Transformation|SetWorldScale3D _staticmesh (* (Math|Vector|MakeVector (Math|Random|RandomFloatinRange 0.8 1.3) (Math|Random|RandomFloatinRange 0.8 1.3) (Math|Random|RandomFloatinRange 0.8 1.3)) (Math|Random|RandomFloatinRange 0.8 1.3))))