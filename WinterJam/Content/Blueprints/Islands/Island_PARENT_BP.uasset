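; Parent Blueprint for islands in a moving-world sailing setup, where islands drift past the ship and act as damaging obstacles.
; A looping timer offsets the island by the PlayerDirection received through MovingWorld_BPI, then expires it once beyond KillDistance from spawn.
; Ship contact triggers EvadeIsland, and a hit also plays a sound and damages TopDownCharacter once until an overlap re-arms it.
; Depleted health opens level "Josef"; the random rotation and scale nodes are unconnected.
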(event OnComponentHit(IslandMesh)
  (params (HitComponent :type Primitive%20Component%20Object%20Reference) (OtherActor :type Actor%20Object%20Reference) (OtherComp :type Primitive%20Component%20Object%20Reference) (NormalImpulse :type Vector :default "0, 0, 0") (Hit :type Hit%20Result%20Structure%20%28by%20ref%29))
  (bind _asship_bp (Utilities|Casting|CastToShip_BP OtherActor))
  (Default|EvadeIsland _asship_bp)
  (Utilities|FlowControl|DoOnce false
    (:Completed
      (Audio|PlaySoundatLocation 0 (Transformation|GetActorLocation self) "0, 0, 0" 1.0 1.0 0.0 0 0 0)
      (CallFunction|CheckandApplyDamage))))

(event OnComponentBeginOverlap(IslandMesh)
  (params (OverlappedComponent :type Primitive%20Component%20Object%20Reference) (OtherActor :type Actor%20Object%20Reference) (OtherComp :type Primitive%20Component%20Object%20Reference) (OtherBodyIndex :type Integer) (bFromSweep :type Boolean) (SweepResult :type Hit%20Result%20Structure%20%28by%20ref%29))
  (bind _asship_bp (Utilities|Casting|CastToShip_BP OtherActor))
  (Default|EvadeIsland _asship_bp)
  (Utilities|FlowControl|DoOnce false) ; enters at Reset
)

(event Custom|CheckKillDistance
  (if (> (Math|Vector|VectorLength (- (Variables|Default|GetSpawnOrigin) (Transformation|GetActorLocation))) (Variables|Default|GetKillDistance))
    (Actor|SetLifeSpan 5.0)))

(event Custom|Move
  (bind _playerdirection (Variables|Default|GetPlayerDirection))
  ;[1 1 1] Called by StartMoving
  (Transformation|AddActorLocalOffset (Math|Vector|MakeVector (.x _playerdirection) (.y _playerdirection) 0.0) false false)
  (CallFunction|CheckKillDistance))

(event EventStartMoving
  ;[1 1 1] Called via MovingWorld_BPI from the ShipBP.
  ;;[1 1 1] Starts/StopsMoving
  (Utilities|FlowControl|DoOnce false
    (:Completed
      (Utilities|Time|SetTimerbyEvent (delegate Custom|Move) 0.05 true))))

(event EventStopMoving
  ;[1 1 1] Called via MovingWorld_BPI from the ShipBP.
  ;;[1 1 1] Starts/StopsMoving
  (Utilities|Time|SetTimerbyEvent (delegate Custom|Move) 0.0)
  (Utilities|FlowControl|DoOnce false) ; enters at Reset
)

(event EventSetPlayerDirection
  (params (PlayerDirection :type Vector :default "0, 0, 0"))
  ;[1 1 1] Called via MovingWorld_BPI from the ShipBP.
  ;;[1 1 1] Get the PlayerDirection from the Interface and Save it as Var
  (Variables|Default|SetPlayerDirection PlayerDirection))

(event EventBeginPlay
  (Variables|Default|SetSpawnOrigin (Transformation|GetActorLocation))
  (CallFunction|StartMoving))

(fn ConstructionScript)

(fn CheckandApplyDamage
  (bind _astop_down_character (Utilities|Casting|CastToTopDownCharacter (Game|GetPlayerCharacter 0)))
  (bind _output_get (Variables|/Game/TopDownBP/Blueprints/TopDownCharacter.TopDownCharacter_C|SetHealth _astop_down_character (Math|Float|Max(Float) (- (Variables|/Game/TopDownBP/Blueprints/TopDownCharacter.TopDownCharacter_C|GetHealth _astop_down_character) 2e+01) 0.0)))
  (Development|PrintString "Schiff ist aufgelaufen")
  (if (<= _output_get 0.0001)
    (Game|OpenLevel(byName) "Josef")
    (Development|PrintString "Hello")))