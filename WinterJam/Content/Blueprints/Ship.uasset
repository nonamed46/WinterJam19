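; Ship actor that the player steers from left and right trigger volumes while it spawns enemies that chase the player.
; Looping timers spawn EnemyCharacters alternately at two spawn points, subject to a live-count cap, and refresh their SimpleMoveToActor orders toward the player.
; TopDownCharacter overlaps with either trigger set a flag and start a timer that rotates the ship in small local steps until the overlap ends.
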(event OnComponentBeginOverlap(Left)
  (params (OverlappedComponent :type Primitive%20Component%20Object%20Reference) (OtherActor :type Actor%20Object%20Reference) (OtherComp :type Primitive%20Component%20Object%20Reference) (OtherBodyIndex :type Integer) (bFromSweep :type Boolean) (SweepResult :type Hit%20Result%20Structure%20%28by%20ref%29))
  ;[0.2965 1 0.7906] Start/Stop turning the Ship Left when overlapping left trigger /ending overlap.
  (Utilities|Casting|CastToTopDownCharacter OtherActor)
  (Variables|Default|SetturnLeft? true)
  (Utilities|Time|SetTimerbyEvent (delegate Custom|TurnLeft) 0.05 (Variables|Default|GetturnLeft?)))

(event OnComponentEndOverlap(Left)
  (params (OverlappedComponent :type Primitive%20Component%20Object%20Reference) (OtherActor :type Actor%20Object%20Reference) (OtherComp :type Primitive%20Component%20Object%20Reference) (OtherBodyIndex :type Integer))
  ;[0.2965 1 0.7906] Start/Stop turning the Ship Left when overlapping left trigger /ending overlap.
  (Utilities|Casting|CastToTopDownCharacter OtherActor)
  (Variables|Default|SetturnLeft? false)
  (Utilities|Time|SetTimerbyEvent (delegate Custom|TurnLeft) 0.0))

(event OnComponentBeginOverlap(Right)
  (params (OverlappedComponent :type Primitive%20Component%20Object%20Reference) (OtherActor :type Actor%20Object%20Reference) (OtherComp :type Primitive%20Component%20Object%20Reference) (OtherBodyIndex :type Integer) (bFromSweep :type Boolean) (SweepResult :type Hit%20Result%20Structure%20%28by%20ref%29))
  ;[0.452 0.6524 1] Start/Stop turning the ship Right when overlapping right trigger /ending overlap.
  (Utilities|Casting|CastToTopDownCharacter OtherActor)
  (Variables|Default|SetturnRight? true)
  (Utilities|Time|SetTimerbyEvent (delegate Custom|TurnRight) 0.05 (Variables|Default|GetturnRight?)))

(event OnComponentEndOverlap(Right)
  (params (OverlappedComponent :type Primitive%20Component%20Object%20Reference) (OtherActor :type Actor%20Object%20Reference) (OtherComp :type Primitive%20Component%20Object%20Reference) (OtherBodyIndex :type Integer))
  ;[0.452 0.6524 1] Start/Stop turning the ship Right when overlapping right trigger /ending overlap.
  (Utilities|Casting|CastToTopDownCharacter OtherActor)
  (Variables|Default|SetturnRight? false)
  (Utilities|Time|SetTimerbyEvent (delegate Custom|TurnRight) 0.0))

(event Custom|SpawnAI
  ;[1 0.3112 0.06219] Spawn AI
  ;;[1 1 1] If there are less then x Enemies alive...
  (bind _outactors (Actor|GetAllActorsOfClass "/Game/TopDownBP/Blueprints/EnemyCharacter.EnemyCharacter_C"))
  (if (<= (Utilities|Array|Length _outactors) 10)
    ;;[1 1 1] ... spawn AI alternating in two locations.
    (Utilities|FlowControl|FlipFlop
      (:A
        (bind _returnvalue (AI|SpawnAIFromClass "/Game/TopDownBP/Blueprints/EnemyCharacter.EnemyCharacter_C" 0 (Transformation|GetWorldLocation (Variables|Default|GetEnemySpawn1)) "0, 0, 0" false))
        (Utilities|IsValid _returnvalue
          (:Is%20Valid
            (AI|Navigation|SimpleMovetoActor (Pawn|GetController _returnvalue) (Game|GetPlayerCharacter 0)))))
      (:B
        (bind _returnvalue_2 (AI|SpawnAIFromClass "/Game/TopDownBP/Blueprints/EnemyCharacter.EnemyCharacter_C" 0 (Transformation|GetWorldLocation (Variables|Default|GetEnemySpawn2)) "0, 0, 0" false))
        (Utilities|IsValid _returnvalue_2
          (:Is%20Valid
            (AI|Navigation|SimpleMovetoActor (Pawn|GetController _returnvalue_2) (Game|GetPlayerCharacter 0))))))))

(event Custom|TurnRight
  ;[0.452 0.6524 1] Start/Stop turning the ship Right when overlapping right trigger /ending overlap.
  (if (Variables|Default|GetturnRight?)
    (Transformation|AddActorLocalRotation self "0,0.100000, 0" false false)))

(event Custom|TurnLeft
  ;[0.2965 1 0.7906] Start/Stop turning the Ship Left when overlapping left trigger /ending overlap.
  (if (Variables|Default|GetturnLeft?)
    (Transformation|AddActorLocalRotation self "0,-0.100000, 0" false false)))

(event Custom|MoveAI
  ;[1 0.002391 0.03508] Moves all AI Actors to the Player
  (bind _outactors (Actor|GetAllActorsOfClass "/Game/TopDownBP/Blueprints/EnemyCharacter.EnemyCharacter_C"))
  (for _array_element _outactors
    (Utilities|IsValid _array_element
      (:Is%20Valid
        (AI|Navigation|SimpleMovetoActor (Pawn|GetController _array_element) (Game|GetPlayerCharacter 0))))))

(event EventBeginPlay
  ;[0.3147 1 0.2994] Setup Event Timers for Spawning and Moving AI
  (Utilities|Time|SetTimerbyEvent (delegate Custom|SpawnAI) 5.0 true)
  (Utilities|Time|SetTimerbyEvent (EventDispatchers|CreateEvent :!event Custom|MoveAI) 0.5 true))

(fn ConstructionScript)