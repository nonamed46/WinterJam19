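; Ship steering Blueprint that keeps a referenced ship actor moving and lets the TopDownCharacter turn it by standing in trigger volumes.
; Tick offsets both the ship and itself by the ship's negated forward vector, applied as a local offset.
; Overlapping the Left or Right trigger starts a looping timer that rotates both actors in small steps.
; Leaving the trigger clears the turn flag and timer.
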(event OnComponentBeginOverlap(Left)
  (params (OverlappedComponent :type Primitive%20Component%20Object%20Reference) (OtherActor :type Actor%20Object%20Reference) (OtherComp :type Primitive%20Component%20Object%20Reference) (OtherBodyIndex :type Integer) (bFromSweep :type Boolean) (SweepResult :type Hit%20Result%20Structure%20%28by%20ref%29))
  ;[1 1 1] Start/Stop turning the Ship Left when overlapping right trigger /ending overlap.
  (Utilities|Casting|CastToTopDownCharacter OtherActor)
  (Variables|Default|SetturnLeft? true)
  (Utilities|Time|SetTimerbyEvent (delegate Custom|TurnLeft) 0.05 (Variables|Default|GetturnLeft?)))

(event OnComponentEndOverlap(Left)
  (params (OverlappedComponent :type Primitive%20Component%20Object%20Reference) (OtherActor :type Actor%20Object%20Reference) (OtherComp :type Primitive%20Component%20Object%20Reference) (OtherBodyIndex :type Integer))
  ;[1 1 1] Start/Stop turning the Ship Left when overlapping right trigger /ending overlap.
  (Utilities|Casting|CastToTopDownCharacter OtherActor)
  (Variables|Default|SetturnLeft? false)
  (Utilities|Time|SetTimerbyEvent (delegate Custom|TurnLeft) 0.0))

(event OnComponentBeginOverlap(Right)
  (params (OverlappedComponent :type Primitive%20Component%20Object%20Reference) (OtherActor :type Actor%20Object%20Reference) (OtherComp :type Primitive%20Component%20Object%20Reference) (OtherBodyIndex :type Integer) (bFromSweep :type Boolean) (SweepResult :type Hit%20Result%20Structure%20%28by%20ref%29))
  ;[1 1 1] Start/Stop turning the ship Right when overlapping right trigger /ending overlap.
  (Utilities|Casting|CastToTopDownCharacter OtherActor)
  (Variables|Default|SetturnRight? true)
  (Utilities|Time|SetTimerbyEvent (delegate Custom|TurnRight) 0.05 (Variables|Default|GetturnRight?)))

(event OnComponentEndOverlap(Right)
  (params (OverlappedComponent :type Primitive%20Component%20Object%20Reference) (OtherActor :type Actor%20Object%20Reference) (OtherComp :type Primitive%20Component%20Object%20Reference) (OtherBodyIndex :type Integer))
  ;[1 1 1] Start/Stop turning the ship Right when overlapping right trigger /ending overlap.
  (Utilities|Casting|CastToTopDownCharacter OtherActor)
  (Variables|Default|SetturnRight? false)
  (Utilities|Time|SetTimerbyEvent (delegate Custom|TurnRight) 0.0))

(event Custom|TurnLeft
  (bind _shi (Variables|Default|GetShi))
  ;[1 1 1] Start/Stop turning the Ship Left when overlapping right trigger /ending overlap.
  (if (Variables|Default|GetturnLeft?)
    (Utilities|IsValid _shi
      (:Is%20Valid
        (Transformation|AddActorLocalRotation _shi "0,-0.100000, 0" false false)))))

(event Custom|TurnRight
  (bind _shi (Variables|Default|GetShi))
  ;[1 1 1] Start/Stop turning the ship Right when overlapping right trigger /ending overlap.
  (if (Variables|Default|GetturnRight?)
    (Utilities|IsValid _shi
      (:Is%20Valid
        (Transformation|AddActorLocalRotation _shi "0,0.100000, 0" false false)))))

(event EventTick
  (params (DeltaSeconds :type Float%20%28single-precision%29))
  (bind _shi (Variables|Default|GetShi))
  (Utilities|IsValid _shi
    (:Is%20Valid
      (Transformation|AddActorLocalOffset _shi (* (Transformation|GetActorForwardVector _shi) -1.0) false false))))

(fn ConstructionScript)